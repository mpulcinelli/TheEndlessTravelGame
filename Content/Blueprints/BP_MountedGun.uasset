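; BP_MountedGun is a mounted gun actor that turns its tripod mesh component to follow the player character.
; Each Tick, and on each target perception update, it sets the component's relative rotation to the look-at rotation from the player's location to the gun's, regardless of what is sensed.
; AI Perception events only print display names, with no firing logic present.
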(event `self.AIPerception.OnPerceptionUpdated`
  (params (UpdatedActors :type "Array of Actor Object Reference (by ref)"))
  (for _array_element UpdatedActors
    (`KismetSystemLibrary.PrintString` (`KismetSystemLibrary.GetDisplayName` _array_element))))

(event `self.AIPerception.OnTargetPerceptionUpdated`
  (params (Actor :type "Actor Object Reference") (Stimulus :type "AIStimulus Structure"))
  (`KismetSystemLibrary.PrintString` (`KismetSystemLibrary.GetDisplayName` null))
  (`SceneComponent.K2_SetRelativeRotation` (`self.MountedGun_Tripod_default_001`) (`KismetMathLibrary.FindLookAtRotation` (`self.K2_GetActorLocation` (`GameplayStatics.GetPlayerCharacter` 0)) (`self.K2_GetActorLocation`)) false false :!label _label))

(event `self.ReceiveTick`
  (params (DeltaSeconds :type "Float (single-precision)"))
  (goto _label))

(fn `UserConstructionScript`)